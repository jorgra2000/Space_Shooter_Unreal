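; BP_Spawner spawns enemies on a repeating Tick timer.
; Each spawn picks from four enemy classes with a random index bounded by the GameMode's Level, so Level controls the variety.
; The transform comes from randomly indexed scene components tagged "Spawn", with a fixed Z height.
; UploadSpawnTime shortens the spawn interval in steps until it reaches a floor, increasing the spawn rate.
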(event `self.ReceiveBeginPlay`
  (bind _asbp_game_mode (cast `/Game/BP_GameMode` (`GameplayStatics.GetGameMode`)))
  (set `self.GameMode` _asbp_game_mode))

(event `self.ReceiveTick`
  (params (DeltaSeconds :type "Float (single-precision)"))
  (set `self.CurrentTimeSpawn` (+ DeltaSeconds (`self.CurrentTimeSpawn`)))
  (if (>= (`self.CurrentTimeSpawn`) (`self.TimeSpawn`))
    (set `self.CurrentTimeSpawn` 0.0)
    (`self.SpawnEnemy`)))

(event `UploadSpawnTime`
  (if (> (`self.TimeSpawn`) 0.5)
    (set `self.TimeSpawn` (- (`self.TimeSpawn`) 0.25))))

(fn `GetClassToSpawn`
  (params (Type :type Integer))
  (returns (Class :type "/Game/Enemies/BP_Enemy Class Reference"))
  (return (select `int` (`KismetMathLibrary.Clamp` Type 0 (`/Game/BP_GameMode.Level` (`self.GameMode`))) :`0` "/Game/Enemies/BP_Enemy.BP_Enemy_C" :`1` "/Game/Enemies/BP_Enemy_Sin.BP_Enemy_Sin_C" :`2` "/Game/Enemies/BP_Enemy_Tank.BP_Enemy_Tank_C" :`3` "/Game/Enemies/BP_Enemy_Double.BP_Enemy_Double_C" :!type "/Game/Enemies/BP_Enemy Class Reference")))

(fn `SpawnEnemy`
  (bind _returnvalue (`self.GetComponentsByTag` "/Script/Engine.SceneComponent" "Spawn"))
  (bind _returnvalue_2 (`SceneComponent.K2_GetComponentToWorld` (`|GetArrayItem` _returnvalue (`KismetMathLibrary.RandomInteger` (`KismetArrayLibrary.Array_Length` _returnvalue)))))
  (bind _class (`self.GetClassToSpawn` (`KismetMathLibrary.RandomInteger` (`/Game/BP_GameMode.Level` (`self.GameMode`)))))
  (`|SpawnActorFromClass` _class (`KismetMathLibrary.MakeTransform` (`KismetMathLibrary.MakeVector` (.x (.location _returnvalue_2)) (.y (.location _returnvalue_2)) 60.0) (.rotation _returnvalue_2) (.scale _returnvalue_2)) "Undefined" "MultiplyWithRoot" null null))

(fn `UserConstructionScript`)
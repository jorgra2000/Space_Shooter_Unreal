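; BP_Enemy is a shooter enemy that flies straight along its initial forward vector and fires bullets from FirePoint on a Tick-accumulated timer.
; Overlaps with BulletPlayer-tagged actors reduce LifePoints; at zero it fires OnEnemyDestroy and notifies BP_GameMode.
; Its bound destroy handler waits briefly, occasionally spawns a fire-speed or triple-shot power-up, then destroys the actor.
; It also destroys itself, without drops, upon leaving a LevelFinal-tagged volume.
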(event `self.ReceiveBeginPlay`
  (set `self.MovementVector` (`self.GetActorForwardVector`))
  (add `self.OnEnemyDestroy` (delegate `DestroyEnemy`)))

(event `DestroyEnemy`
  (bind _returnvalue (`self.GetTransform`))
  (`KismetSystemLibrary.Delay` 0.1)
  (if (>= (`KismetMathLibrary.RandomFloat`) 0.9)
    (if (>= (`KismetMathLibrary.RandomFloat`) 0.5)
      (`|SpawnActorFromClass` "/Game/PowerUps/BP_PowerUp_FireSpeed.BP_PowerUp_FireSpeed_C" _returnvalue "Undefined" "MultiplyWithRoot" null null)
      (else
        (`|SpawnActorFromClass` "/Game/PowerUps/BP_PoweUp_TripleShoot.BP_PoweUp_TripleShoot_C" _returnvalue "Undefined" "MultiplyWithRoot" null null))))
  (`self.K2_DestroyActor`))

(event `self.ReceiveActorBeginOverlap`
  (params (OtherActor :type "Actor Object Reference"))
  ;[1 1 1] Collision
  (if (`KismetArrayLibrary.Array_Contains` (`Actor.Tags` OtherActor) "BulletPlayer")
    (set `self.LifePoints` (- (`self.LifePoints`) 1))
    (if (<= (`self.LifePoints`) 0)
      (`self.OnEnemyDestroy`)
      (bind _asbp_game_mode (cast `/Game/BP_GameMode` (`GameplayStatics.GetGameMode`)))
      (`/Game/BP_GameMode.EnemyDestroy` _asbp_game_mode))))

(event `self.ReceiveTick`
  (params (DeltaSeconds :type "Float (single-precision)"))
  ;[1 1 1] Move and Shoot
  (`self.Move` DeltaSeconds)
  (bind _output_get (set `self.ShootCurrentTime` (+ DeltaSeconds (`self.ShootCurrentTime`))))
  (if (>= _output_get (`self.FireDelay`))
    (set `self.ShootCurrentTime` 0.0)
    (`self.Shoot`)))

(event `self.ReceiveActorEndOverlap`
  (params (OtherActor :type "Actor Object Reference"))
  (if (`KismetArrayLibrary.Array_Contains` (`Actor.Tags` OtherActor) "LevelFinal")
    (`self.K2_DestroyActor`)))

(fn `Move`
  (params (DeltaTime :type "Float (double-precision)"))
  (`self.K2_SetActorLocation` (+ (`self.K2_GetActorLocation`) (* (* DeltaTime (`self.Speed`)) (`self.MovementVector`)))))

(fn `Shoot`
  (`|SpawnActorFromClass` (`self.Bullet`) (`SceneComponent.K2_GetComponentToWorld` (`self.FirePoint`)) "Undefined" "MultiplyWithRoot" null null))

(fn `UserConstructionScript`)
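; Enemy Blueprint that moves in a sine-wave pattern and fires on a repeating timer.
; Tick calls MoveSin, then accumulates time and calls Shoot whenever FireDelay elapses.
; MoveSin advances X by Speed and MovementVector and locks Z at a constant height.
; Y gains a sine offset from accumulated time, Frequency and Amplitude each frame without delta-time scaling, so the sway depends on frame rate.
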(event `self.ReceiveTick`
  (params (DeltaSeconds :type "Float (single-precision)"))
  (`self.MoveSin` DeltaSeconds)
  (bind _output_get (set `self.ShootCurrentTime` (+ DeltaSeconds (`self.ShootCurrentTime`))))
  (if (>= _output_get (`self.FireDelay`))
    (set `self.ShootCurrentTime` 0.0)
    (`self.Shoot`)))

(fn `MoveSin`
  (params (DeltaTime :type "Float (double-precision)"))
  (bind _returnvalue (`self.K2_GetActorLocation`))
  (bind _returnvalue_x (`KismetMathLibrary.BreakVector` (+ _returnvalue (* (* DeltaTime (`self.Speed`)) (`self.MovementVector`)))))
  (bind _output_get (set `self.TimeAcum` (+ DeltaTime (`self.TimeAcum`))))
  (bind (_returnvalue_x_2 _returnvalue_y) (`KismetMathLibrary.BreakVector` (+ _returnvalue (* (`KismetMathLibrary.Sin` (* _output_get (`self.Frequency`))) (`self.Amplitude`)))))
  (`self.K2_SetActorLocation` (`KismetMathLibrary.MakeVector` _returnvalue_x _returnvalue_y 60.0)))

(fn `UserConstructionScript`
  (`parent.UserConstructionScript`))
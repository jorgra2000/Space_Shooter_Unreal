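; Bullet projectile actor that flies straight along its forward vector and explodes on overlap.
; Tick moves it by Speed scaled by delta time, setting location without sweep.
; Any actor overlap spawns an explosion particle and 2D sound at its location, then destroys the bullet after a short delay.
; The graph applies no damage and does not filter what it overlaps.
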(event `self.ReceiveActorBeginOverlap`
  (params (OtherActor :type "Actor Object Reference"))
  (`GameplayStatics.SpawnEmitterAtLocation` "/Game/P_BulletExplosion.P_BulletExplosion" (`self.K2_GetActorLocation`))
  (`GameplayStatics.PlaySound2D` "/Game/StarterContent/Audio/Explosion01.Explosion01" 0.35 1.0 0.0 null null)
  (`KismetSystemLibrary.Delay` 0.1)
  (`self.K2_DestroyActor`))

(event `self.ReceiveTick`
  (params (DeltaSeconds :type "Float (single-precision)"))
  ;[1 1 1] Bullet movement
  (`self.K2_SetActorLocation` (+ (`self.K2_GetActorLocation`) (* (`self.GetActorForwardVector`) (* DeltaSeconds (`self.Speed`))))))

(fn `UserConstructionScript`)
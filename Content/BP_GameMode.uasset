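; Game mode for a shooter that plays the main theme at start and tracks score, difficulty level and game over.
; Each destroyed enemy adds points, and every multiple of 50 raises the level up to a cap and tells BP_Spawner to update its spawn time.
; Player death triggers the end-game screen on BP_HUD, and power-up events start or stop the FireSpeed and TripleShoot displays there by name.
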(event `self.ReceiveBeginPlay`
  (`GameplayStatics.PlaySound2D` "/Game/Main_theme.Main_theme" 0.5 1.0 0.0 null null))

(event `self.ReceiveTick`
  (params (DeltaSeconds :type "Float (single-precision)")))

(event `EnemyDestroy`
  (bind _level (`self.Level`))
  (set `self.Points` (+ (`self.Points`) (`self.IncremetPoints`)))
  (if (== (mod (`self.Points`) 50) 0)
    (if (<= _level 4)
      (set `self.Level` (+ _level 1))
      (bind _returnvalue (`GameplayStatics.GetActorOfClass` "/Game/BP_Spawner.BP_Spawner_C"))
      (`/Game/BP_Spawner.UploadSpawnTime` _returnvalue))))

(event `PlayerDead`
  (bind _asbp_hud (cast `/Game/BP_HUD` (`PlayerController.GetHUD` (`GameplayStatics.GetPlayerController` 0))))
  (`/Game/BP_HUD.EndGame` _asbp_hud))

(event `ActivatePowerUp`
  (params (Name :type String))
  (bind _returnvalue (`PlayerController.GetHUD` (`GameplayStatics.GetPlayerController` 0)))
  ;[1 1 1] Activate Power Up
  (if (`KismetStringLibrary.EqualEqual_StrStr` Name "FireSpeed")
    (bind _asbp_hud (cast `/Game/BP_HUD` _returnvalue))
    (`/Game/BP_HUD.Start_PU_FireSpeed` _asbp_hud)
    (elif (`KismetStringLibrary.EqualEqual_StrStr` Name "TripleShoot")
      (bind _asbp_hud_2 (cast `/Game/BP_HUD` _returnvalue))
      (`/Game/BP_HUD.Start_PU_TripleShoot` _asbp_hud_2))))

(event `DisablePowerUp`
  (params (Name :type String))
  (bind _returnvalue (`PlayerController.GetHUD` (`GameplayStatics.GetPlayerController` 0)))
  ;[1 1 1] Disable Power Up
  (if (`KismetStringLibrary.EqualEqual_StrStr` Name "FireSpeed")
    (bind _asbp_hud (cast `/Game/BP_HUD` _returnvalue))
    (`/Game/BP_HUD.Stop_PU_FireSpeed` _asbp_hud)
    (elif (`KismetStringLibrary.EqualEqual_StrStr` Name "TripleShoot")
      (bind _asbp_hud_2 (cast `/Game/BP_HUD` _returnvalue))
      (`/Game/BP_HUD.Stop_PU_TripleShoot` _asbp_hud_2))))

(fn `UserConstructionScript`)